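; BP_Color_Light_Puzzle controls a combination puzzle made of four BP_Color_Light child actors.
; On BeginPlay it caches each light, passes itself as its PuzzleControl and assigns hardcoded goal numbers.
; CheckComplete, which nothing in this graph calls, compares every light's current number to its goal.
; When all match, it turns the lights green, deactivates them and sets OpenDoorM on the player.
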(event `self.ReceiveBeginPlay`
  (bind _asbp_color_light (cast `/Game/01_MAIN_Project/Blueprints/Item/BP_Color_Light` (`ChildActorComponent.ChildActor` (`self.Light1`))))
  (bind _output_get (set `self.ColorLight1` _asbp_color_light))
  (set `/Game/01_MAIN_Project/Blueprints/Item/BP_Color_Light.Puzzle Control` self _output_get)
  (bind _asbp_color_light_2 (cast `/Game/01_MAIN_Project/Blueprints/Item/BP_Color_Light` (`ChildActorComponent.ChildActor` (`self.Light2`))))
  (bind _output_get_2 (set `self.ColorLight2` _asbp_color_light_2))
  (set `/Game/01_MAIN_Project/Blueprints/Item/BP_Color_Light.Puzzle Control` self _output_get_2)
  (bind _asbp_color_light_3 (cast `/Game/01_MAIN_Project/Blueprints/Item/BP_Color_Light` (`ChildActorComponent.ChildActor` (`self.Light3`))))
  (bind _output_get_3 (set `self.ColorLight3` _asbp_color_light_3))
  (set `/Game/01_MAIN_Project/Blueprints/Item/BP_Color_Light.Puzzle Control` self _output_get_3)
  (bind _asbp_color_light_4 (cast `/Game/01_MAIN_Project/Blueprints/Item/BP_Color_Light` (`ChildActorComponent.ChildActor` (`self.Light4`))))
  (bind _output_get_4 (set `self.ColorLight4` _asbp_color_light_4))
  (set `/Game/01_MAIN_Project/Blueprints/Item/BP_Color_Light.Puzzle Control` self _output_get_4)
  (`self.SetGoalNums`))

(fn `CheckComplete`
  (bind _colorlight2 (`self.ColorLight2`))
  (bind _colorlight3 (`self.ColorLight3`))
  (bind _colorlight4 (`self.ColorLight4`))
  (bind _colorlight1 (`self.ColorLight1`))
  (if (== (`/Game/01_MAIN_Project/Blueprints/Item/BP_Color_Light.Current Number` _colorlight1) (`/Game/01_MAIN_Project/Blueprints/Item/BP_Color_Light.Goal Number` _colorlight1))
    (if (== (`/Game/01_MAIN_Project/Blueprints/Item/BP_Color_Light.Current Number` _colorlight2) (`/Game/01_MAIN_Project/Blueprints/Item/BP_Color_Light.Goal Number` _colorlight2))
      (if (== (`/Game/01_MAIN_Project/Blueprints/Item/BP_Color_Light.Current Number` _colorlight3) (`/Game/01_MAIN_Project/Blueprints/Item/BP_Color_Light.Goal Number` _colorlight3))
        (if (== (`/Game/01_MAIN_Project/Blueprints/Item/BP_Color_Light.Current Number` _colorlight4) (`/Game/01_MAIN_Project/Blueprints/Item/BP_Color_Light.Goal Number` _colorlight4))
          (`self.OnPuzzleSolve`)
          (bind _asbp_player (cast `/Game/01_MAIN_Project/Blueprints/BP_Player` (`GameplayStatics.GetPlayerPawn` 0)))
          (set `/Game/01_MAIN_Project/Blueprints/BP_Player.OpenDoorM` true _asbp_player))))))

(fn `OnPuzzleSolve`
  (bind _colorlight2 (`self.ColorLight2`))
  (bind _colorlight3 (`self.ColorLight3`))
  (bind _colorlight4 (`self.ColorLight4`))
  (bind _colorlight1 (`self.ColorLight1`))
  (`LightComponent.SetLightColor` (`/Game/01_MAIN_Project/Blueprints/Item/BP_Color_Light.PointLight` _colorlight1) (struct :`R` 0.012024 :`G` 0.458333 :`A` 1.0) true)
  (set `/Game/01_MAIN_Project/Blueprints/Item/BP_Color_Light.Active` false _colorlight1)
  (`LightComponent.SetLightColor` (`/Game/01_MAIN_Project/Blueprints/Item/BP_Color_Light.PointLight` _colorlight2) (struct :`R` 0.012024 :`G` 0.458333 :`A` 1.0) true)
  (set `/Game/01_MAIN_Project/Blueprints/Item/BP_Color_Light.Active` false _colorlight2)
  (`LightComponent.SetLightColor` (`/Game/01_MAIN_Project/Blueprints/Item/BP_Color_Light.PointLight` _colorlight3) (struct :`R` 0.012024 :`G` 0.458333 :`A` 1.0) true)
  (set `/Game/01_MAIN_Project/Blueprints/Item/BP_Color_Light.Active` false _colorlight3)
  (`LightComponent.SetLightColor` (`/Game/01_MAIN_Project/Blueprints/Item/BP_Color_Light.PointLight` _colorlight4) (struct :`R` 0.012024 :`G` 0.458333 :`A` 1.0) true)
  (set `/Game/01_MAIN_Project/Blueprints/Item/BP_Color_Light.Active` false _colorlight4))

(fn `SetGoalNums`
  (set `/Game/01_MAIN_Project/Blueprints/Item/BP_Color_Light.Goal Number` 1 (`self.ColorLight1`))
  (set `/Game/01_MAIN_Project/Blueprints/Item/BP_Color_Light.Goal Number` 7 (`self.ColorLight2`))
  (set `/Game/01_MAIN_Project/Blueprints/Item/BP_Color_Light.Goal Number` 3 (`self.ColorLight3`))
  (set `/Game/01_MAIN_Project/Blueprints/Item/BP_Color_Light.Goal Number` 4 (`self.ColorLight4`)))

(fn `UserConstructionScript`)