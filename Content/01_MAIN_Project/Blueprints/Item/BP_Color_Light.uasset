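; BP_Color_Light is an interactable puzzle light whose color the player cycles through.
; When active and used by BP_Player, it advances an index through eight preset colors, applies the matching one to its PointLight and asks PuzzleControl to check completion.
; BeginPlay stores the light's current color as the starting Color without deriving the index from it.
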(event `self.ReceiveBeginPlay`
  (set `self.Color` (`LightComponentBase.GetLightColor` (`self.PointLight`))))

(event `/Game/01_MAIN_Project/Blueprints/Interact_Interface.Interact`
  (params (Interactor :type "Actor Object Reference"))
  (if (`self.Active`)
    (cast `/Game/01_MAIN_Project/Blueprints/BP_Player` Interactor)
    (set `self.Current Number` (mod (+ (`self.Current Number`) 1) 8))
    (`self.UpdateLightColor`)
    (`/Game/01_MAIN_Project/Blueprints/Item/BP_Color_Light_Puzzle.CheckComplete` (`self.Puzzle Control`))))

(fn `UpdateLightColor`
  (switch `int` (`self.Current Number`)
    (:`0`
      (set `self.Color` (struct :`R` 1.0 :`G` 0.352941 :`A` 1.0)))
    (:`1`
      (set `self.Color` (struct :`R` 0.159453 :`B` 1.0 :`A` 1.0)))
    (:`2`
      (set `self.Color` (struct :`G` 0.057209 :`B` 1.0 :`A` 1.0)))
    (:`3`
      (set `self.Color` (struct :`R` 1.0 :`B` 0.05342 :`A` 1.0)))
    (:`4`
      (set `self.Color` (struct :`R` 1.0 :`G` 0.824953 :`A` 1.0)))
    (:`5`
      (set `self.Color` (struct :`G` 0.943338 :`B` 1.0 :`A` 1.0)))
    (:`6`
      (set `self.Color` (struct :`R` 1.0 :`G` 0.203125 :`B` 0.806869 :`A` 1.0)))
    (:`7`
      (set `self.Color` (struct :`R` 0.090742 :`G` 1.0 :`A` 1.0))))
  (`LightComponent.SetLightColor` (`self.PointLight`) (`self.Color`) true))

(fn `UserConstructionScript`)