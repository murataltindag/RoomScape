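; Base pickup item actor that can be collected into an inventory or brought up for inspection.
; Interact adds a slot built from its item structure to the interactor's InventoryComponent and destroys the actor on success.
; StartInspect disables the player's input, calls EnableInput on the player controller and moves the item a fixed distance in front of the camera.
; UseItem is a stub that returns false.
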(event `/Game/01_MAIN_Project/Blueprints/Interact_Interface.Interact`
  (params (Interactor :type "Actor Object Reference"))
  (bind _success (`/Game/01_MAIN_Project/Blueprints/InventoryComponent.addToInventory` (`self.GetComponentByClass` Interactor "/Game/01_MAIN_Project/Blueprints/InventoryComponent.InventoryComponent_C") (make `/Game/01_MAIN_Project/Blueprints/SlotStructure` (`self.ItemStructure`))))
  (if _success
    (`self.K2_DestroyActor`)))

(fn `Start Inspect`
  (bind _returnvalue (`GameplayStatics.GetPlayerController` 0))
  (bind _returnvalue_2 (`GameplayStatics.GetPlayerCameraManager` 0))
  (`self.DisableInput` (`self.Player`) _returnvalue)
  (`self.EnableInput` _returnvalue null)
  (`self.K2_SetActorLocation` (+ (`PlayerCameraManager.GetCameraLocation` _returnvalue_2) (* (`KismetMathLibrary.GetForwardVector` (`PlayerCameraManager.GetCameraRotation` _returnvalue_2)) 200.0))))

(fn `UseItem`
  (returns (Success :type Boolean))
  (return false))

(fn `UserConstructionScript`)