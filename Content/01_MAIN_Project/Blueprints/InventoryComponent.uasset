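; Inventory component that stores items in a fixed number of slots and toggles an inventory window for its local player.
; Slots are sized on BeginPlay; adding writes into the first empty slot, without merging stacks, and always reports success.
; Toggling adds the window to player 0's HUD canvas, left or right by player index.
; It also sets that player's Paused flag and switches input mode.
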(event `self.ReceiveBeginPlay`
  (`self.prepareInventory`))

(fn `addToInventory`
  (params (ContentsToAdd :type "/Game/01_MAIN_Project/Blueprints/SlotStructure Structure"))
  (returns (Success :type Boolean))
  (`self.CreateStack` ContentsToAdd)
  (return true))

(fn `CreateStack`
  (params (ContenttoAdd :type "/Game/01_MAIN_Project/Blueprints/SlotStructure Structure"))
  (bind _inventory (`self.Inventory`))
  (`KismetArrayLibrary.Array_Set` _inventory (`KismetArrayLibrary.Array_Find` _inventory (make `/Game/01_MAIN_Project/Blueprints/SlotStructure` (struct :`Name` "NSLOCTEXT(\"[A4B82BEB4B3BFA6383493F9970285480]\", \"B7E515594E3AB67CA92E249E63A6B6C9\", \"None\")" :`Description` "NSLOCTEXT(\"[A4B82BEB4B3BFA6383493F9970285480]\", \"EC54E575421B4B482848B08D02E6B494\", \"None\")"))) ContenttoAdd))

(fn `GetInventoryPosition`
  (params (Divide :type Integer))
  (returns (Position :type "Float (double-precision)"))
  (return (`KismetMathLibrary.Conv_IntToDouble` (/ (`PlayerController.GetViewportSize` (`GameplayStatics.GetPlayerController` (`self.PlayerContoller`))) Divide))))

(fn `prepareInventory`
  (`KismetArrayLibrary.Array_Resize` (`self.Inventory`) (`self.NumberOfSlots`)))

(fn `ToggleInventory`
  (bind _alignx (`self.AlignX`))
  (bind _playercontoller (`self.PlayerContoller`))
  (`self.InventoryWindow`
    (:`then`
      (`Widget.RemoveFromParent` (`self.InventoryWindow`))
      (set `self.InventoryWindow` null)
      (bind _asbp_player (cast `/Game/01_MAIN_Project/Blueprints/BP_Player` (`GameplayStatics.GetPlayerCharacter` (`self.PlayerContoller`))))
      (set `/Game/01_MAIN_Project/Blueprints/BP_Player.Paused` false _asbp_player)
      (`WidgetBlueprintLibrary.SetInputMode_GameOnly` (`GameplayStatics.GetPlayerController` (`self.PlayerContoller`))))
    (:`else`
      (bind _returnvalue (`|CreateWidget` "/Game/01_MAIN_Project/UI/InventoryUI/InventoryWindow.InventoryWindow_C" null self))
      (set `self.InventoryWindow` _returnvalue)
      (bind _asmy_player_controller (cast `/Game/01_MAIN_Project/Blueprints/MyPlayerController` (`GameplayStatics.GetPlayerController` 0)))
      (bind _returnvalue_2 (`CanvasPanel.AddChildToCanvas` (`/Game/01_MAIN_Project/UI/InventoryUI/HUD.Hud_canvas` (`/Game/01_MAIN_Project/Blueprints/MyPlayerController.hud_widget` _asmy_player_controller)) (`self.InventoryWindow`)))
      (`CanvasPanelSlot.SetAutoSize` _returnvalue_2 true)
      (if (`KismetMathLibrary.Conv_IntToBool` (`self.PlayerContoller`))
        (set `self.AlignX` 0.75)
        (else
          (set `self.AlignX` 0.25)))
      (`CanvasPanelSlot.SetAnchors` _returnvalue_2 (make `Anchors` (`KismetMathLibrary.MakeVector2D` _alignx 0.5) (`KismetMathLibrary.MakeVector2D` _alignx 0.5)))
      (`CanvasPanelSlot.SetAlignment` _returnvalue_2 (0.5 0.5))
      (bind _asbp_player_2 (cast `/Game/01_MAIN_Project/Blueprints/BP_Player` (`GameplayStatics.GetPlayerCharacter` _playercontoller)))
      (set `/Game/01_MAIN_Project/Blueprints/BP_Player.Paused` true _asbp_player_2)
      (`WidgetBlueprintLibrary.SetInputMode_GameAndUIEx` (`GameplayStatics.GetPlayerController` _playercontoller) (`self.InventoryWindow`) "LockAlways" false))))